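; RTS player controller that handles camera movement, unit selection and move orders.
; Axis input moves the controlled pawn along control yaw, falling back to screen-edge mouse scrolling when no axis input is given.
; Left mouse starts and stops RTS_HUD selection drawing, clearing selected units and building on press.
; Selections arrive through events; MouseClick release sends selected units to the cursor hit via BPI_UnitActions, drawing debug spheres there.
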(event Custom|UnitSelectionFinished
  (params (SelectedActor :type Actor%20Object%20Reference))
  ;[1 1 1] Adding units to array
  (Utilities|Array|Add (Variables|Default|GetSelectedUnits) SelectedActor))

(event Custom|BuildingClicked
  (params (SelectedBuilding :type BP%20Building%20Object%20Reference))
  ;[1 1 1] Setting selected building var
  (Variables|Default|SetSelectedBuilding SelectedBuilding))

(event EventBeginPlay
  (Development|PrintString "Game Started")
  (bind _asrts_hud (Utilities|Casting|CastToRTS_HUD (HUD|GetHUD)))
  (Variables|Default|SetHUDref _asrts_hud))

(event EventTick
  (params (DeltaSeconds :type Float%20%28single-precision%29)))

(event Input|ActionEvents|InputActionDebuggingControl
  (params (Key :type Key%20Structure :default "None"))
  ;[1 1 1] MouseControlImplementation
  (:Pressed
    (bind _output_get (Variables|Default|SetDebugModeToggle (== (Variables|Default|GetDebugModeToggle) false)))))

(event Input|ActionEvents|InputActionMouseClick
  (params (Key :type Key%20Structure :default "None"))
  (bind _hitresult (Game|Player|GetHitResultUnderCursorbyChannel "TraceTypeQuery1" true))
  (bind _location (Collision|BreakHitResult _hitresult))
  (:Released
    (if (Utilities|Array|IsNotEmpty (Variables|Default|GetSelectedUnits))
      (for _array_element (Variables|Default|GetSelectedUnits)
        (if (Utilities|DoesObjectImplementInterface _array_element "/Game/RTS/Core/Unit/BPI_UnitActions.BPI_UnitActions_C")
          (Class|BPIUnitActions|MovetoLocation(Message) _array_element _location)
          (Rendering|Debug|DrawDebugSphere _location 3e+01 12 "(R=0.807292,G=0.042046,B=0.049503,A=1.000000)" 5.0 1.0))))))

(event Input|AxisEvents|InputAxisMoveVertical
  (params (AxisValue :type Float%20%28single-precision%29))
  ;[1 1 1] CameraMovement
  (Pawn|Input|AddMovementInput (Pawn|GetControlledPawn) (Math|Vector|GetForwardVector (Math|Rotator|MakeRotator 0.0 0.0 (.yaw (Pawn|GetControlRotation :!class /Script/Engine.Controller)))) (Math|Float|SelectFloat AxisValue (Variables|Default|GetMouseForwardScale) (or (!= AxisValue 0.0) (!= (stale Input|AxisEvents|InputAxisMoveHorizontal AxisValue) 0.0))) false))

(event Input|AxisEvents|InputAxisMoveHorizontal
  (params (AxisValue :type Float%20%28single-precision%29))
  ;[1 1 1] CameraMovement
  (Pawn|Input|AddMovementInput (Pawn|GetControlledPawn) (Math|Vector|GetRightVector (Math|Rotator|MakeRotator 0.0 0.0 (.yaw (Pawn|GetControlRotation :!class /Script/Engine.Controller)))) (Math|Float|SelectFloat AxisValue (Variables|Default|GetMouseRightScale) (or (!= (stale Input|AxisEvents|InputAxisMoveVertical AxisValue) 0.0) (!= AxisValue 0.0))) false))

(event Input|AxisEvents|InputAxisMouseMovement
  (params (AxisValue :type Float%20%28single-precision%29))
  (bind _locationy (Game|Player|GetMousePosition))
  (bind _returnvalue (Viewport|GetViewportSize))
  (bind (_locationx _locationy_2) (Game|Player|GetMousePosition))
  (bind _returnvalue_2 (Viewport|GetViewportSize))
  (bind _locationx_2 (Game|Player|GetMousePosition))
  (bind _returnvalue_3 (Viewport|GetViewportSize))
  (bind _viewportedgethrashold (Variables|Default|GetViewportEdgeThrashold))
  (bind _viewportedgethrashold_2 (Variables|Default|GetViewportEdgeThrashold))
  (bind _returnvalue_4 (/ _locationy (.y _returnvalue)))
  (bind _returnvalue_5 (/ _locationx_2 (.x _returnvalue_3)))
  ;[1 1 1] MouseControlImplementation
  (Development|PrintString (Utilities|String|Append (Utilities|String|ToString(Float) (/ _locationx (.x _returnvalue_2))) ", " (Utilities|String|ToString(Float) (/ _locationy_2 (.y _returnvalue_2)))) (stale Input|ActionEvents|InputActionDebuggingControl _output_get) true "(R=0.000000,G=0.187500,B=0.043678,A=1.000000)" 0.0)
  (Variables|Default|SetMouseRightScale (Math|Float|SelectFloat -1.0 (Math|Float|SelectFloat 1.0 0.0 (> _returnvalue_5 (- 1.0 _viewportedgethrashold_2))) (< _returnvalue_5 _viewportedgethrashold_2)))
  (Variables|Default|SetMouseForwardScale (Math|Float|SelectFloat 1.0 (Math|Float|SelectFloat -1.0 0.0 (> _returnvalue_4 (- 1.0 _viewportedgethrashold))) (< _returnvalue_4 _viewportedgethrashold))))

(event Input|MouseEvents|LeftMouseButton
  (params (Key :type Key%20Structure :default "None"))
  (bind _hudref (Variables|Default|GetHUDref))
  ;[1 1 1] Start/stop multiselecting management
  (:Pressed
    (Utilities|FlowControl|Sequence
      (:then_0
        (Utilities|IsValid (Variables|Default|GetSelectedBuilding)
          (:Is%20Valid
            (Default|BuildingDeselected (Variables|Default|GetSelectedBuilding))
            (Variables|Default|SetSelectedBuilding 0))
          (:Is%20Not%20Valid
            (Default|StartDraw _hudref :!label _label))))
      (:then_1
        (Utilities|Array|Clear (Variables|Default|GetSelectedUnits))
        (goto _label))))
  (:Released
    (Default|StopDraw _hudref)))

(fn ConstructionScript)