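; BP_UnitComponent is an actor component that makes its owning RTS unit click-selectable.
; On BeginPlay it caches the owner and its DecalComponent, then binds to the owner's OnClicked event.
; Selection reports the unit to PC_RTS through UnitSelectionFinished and shows the decal as a selection marker, while UnitDeselected hides it again.
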(event Custom|OnUnitClicked
  (params (TouchedActor :type Actor%20Object%20Reference) (ButtonPressed :type Key%20Structure :default "None"))
  ;[1 1 1] Unit selection
  (CallFunction|UnitSelected))

(event Custom|UnitDeselected
  ;[1 1 1] Unit selection
  (Development|SetHiddeninGame (Variables|Default|GetSelectionDecal) true false))

(event Custom|UnitSelected
  ;[1 1 1] Unit selection
  (Utilities|FlowControl|Sequence
    (:then_0
      (bind _aspc_rts (Utilities|Casting|CastToPC_RTS (Game|GetPlayerController 0)))
      (Default|UnitSelectionFinished _aspc_rts (Variables|Default|GetThisUnit)))
    (:then_1
      (Development|SetHiddeninGame (Variables|Default|GetSelectionDecal) false false))))

(event EventBeginPlay
  (bind _returnvalue (Components|GetOwner))
  ;[1 1 1] Getting ref to unit, his components and event
  (bind _output_get (Variables|Default|SetThisUnit _returnvalue))
  (Variables|Default|SetSelectionDecal (Actor|GetComponentbyClass _returnvalue "/Script/Engine.DecalComponent"))
  (EventDispatchers|BindEventtoOnClicked _output_get (EventDispatchers|CreateEvent :!event Custom|OnUnitClicked)))