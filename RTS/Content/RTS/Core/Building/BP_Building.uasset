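; BP_Building is an RTS building actor that handles selection by mouse click.
; A left click waits briefly, then fires BuildingSelected, which passes the building to PC_RTS through BuildingClicked and reveals its selection decal.
; A separate BuildingDeselected event hides the decal, with no caller inside this Blueprint.
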(event Custom|BuildingSelected
  (Utilities|FlowControl|Sequence
    (:then_0
      (bind _aspc_rts (Utilities|Casting|CastToPC_RTS (Game|GetPlayerController 0)))
      (Default|BuildingClicked _aspc_rts self))
    (:then_1
      (Development|SetHiddeninGame (Variables|Default|GetSelectionDecal) false false))))

(event Custom|BuildingDeselected
  (Development|SetHiddeninGame (Variables|Default|GetSelectionDecal) true false))

(event EventBeginPlay)

(event Collision|EventActorBeginOverlap
  (params (OtherActor :type Actor%20Object%20Reference)))

(event EventTick
  (params (DeltaSeconds :type Float%20%28single-precision%29)))

(event MouseInput|EventActorOnClicked
  (params (ButtonPressed :type Key%20Structure :default "None"))
  (if (== ButtonPressed "LeftMouseButton")
    (Utilities|FlowControl|Delay 0.1)
    (CallFunction|BuildingSelected)))

(fn ConstructionScript)